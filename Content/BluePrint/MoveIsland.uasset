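; MoveIsland is an actor Blueprint that moves itself back and forth between its starting location and the location of a referenced FinishActor.
; Tick advances an alpha by scaled delta time and lerps the actor's location between the two endpoints.
; Within a small tolerance of the target, it swaps the endpoints, resets alpha and sets a flag that triggers a short Delay before the return trip.
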(event EventBeginPlay
  (Variables|Default|SetStartLoc (Transformation|GetActorLocation))
  (Variables|Default|SetFinishLoc (Transformation|GetActorLocation (Variables|Default|GetFinishActor))))

(event EventTick
  (params (DeltaSeconds :type Float%20%28single-precision%29))
  (if (Variables|Default|GetDelayBool)
    (Utilities|FlowControl|Delay 3.0)
    (Variables|Default|SetDelayBool false))
  (bind _output_get (Variables|Default|SetAlpha (+ (/ DeltaSeconds 1e+01) (Variables|Default|GetAlpha))))
  (bind _output_get_2 (Variables|Default|SetCurrentLoc (Math|Vector|Lerp(Vector) (Variables|Default|GetStartLoc) (Variables|Default|GetFinishLoc) _output_get)))
  (if (Utilities|Operators|EqualEqual _output_get_2 (Variables|Default|GetFinishLoc) 1e+01)
    (Variables|Default|SetCurrentLoc (Variables|Default|GetFinishLoc))
    (Variables|Default|SetFinishLoc (Variables|Default|GetStartLoc))
    (Variables|Default|SetStartLoc (Variables|Default|GetCurrentLoc))
    (Variables|Default|SetAlpha 0.0)
    (Variables|Default|SetDelayBool true)
    (else
      (Transformation|SetActorLocation (Variables|Default|GetCurrentLoc) false false))))

(fn ConstructionScript)